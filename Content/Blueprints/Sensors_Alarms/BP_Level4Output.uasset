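; BP_Level4Output is an interactable lever that signals up to four linked output actors.
; Interacting plays a sound, then sends InteractMessage to all four actors, though only the primary OutputActor is checked for validity and BPI_Interact.
; It then toggles Activated and plays or reverses the PullLever timeline to rotate the lever.
; The toggle and animation run only if that primary check passes.
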(event `self.Interact`
  (`self.Switch Lever`))

(event `Switch Lever`
  (`GameplayStatics.PlaySoundAtLocation` "/Engine/VREditor/Sounds/UI/Floating_UI_Close.Floating_UI_Close" (`self.K2_GetActorLocation`) (struct) 1.0 1.0 0.0 "/Game/Audio/Alarms/SA_Sensor.SA_Sensor" null null null)
  (bind _output_actor (`self.output Actor`)
    (:`then`
      (if (`KismetSystemLibrary.DoesImplementInterface` _output_actor "/Game/Blueprints/BPI_Interact.BPI_Interact_C")
        (`|ExecutionSequence`
          (:`then_0`
            (message `/Game/Blueprints/BPI_Interact.Interact` (`self.output Actor 2`)))
          (:`then_1`
            (message `/Game/Blueprints/BPI_Interact.Interact` (`self.output Actor 3`)))
          (:`then_2`
            (message `/Game/Blueprints/BPI_Interact.Interact` (`self.output Actor 4`)))
          (:`then_3`
            (message `/Game/Blueprints/BPI_Interact.Interact` _output_actor)
            (if (not (`self.activated`))
              (set `self.activated` true)
              (bind (_direction _rotation) (`Timeline|Pull Lever` :!label _label)
                (:`Update`
                  (`SceneComponent.K2_SetRelativeRotation` (`self.Lever`) (`KismetMathLibrary.RLerp` (struct :`Pitch` 120.0) (struct :`Pitch` 50.0) _rotation) false false)))
              (else
                (set `self.activated` false)
                (goto _label :!via `Reverse`)))))))
    (:`else`)))

(fn `UserConstructionScript`)