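; A toggleable point light actor, filed with sensors and alarms, that responds to an Interact event.
; Interact checks the Activated flag, then flips it along with the PointLight's visibility.
; It also switches the whole actor's collision to match, enabled when lit and disabled when off.
; The construction script only calls its parent, and BeginPlay, overlap and Tick are unused.
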(event `self.Interact`
  (if (not (`self.activated`))
    (`self.SetActorEnableCollision` true)
    (`SceneComponent.SetVisibility` (`self.PointLight`) true false)
    (set `self.activated` true)
    (else
      (`self.SetActorEnableCollision` false)
      (`SceneComponent.SetVisibility` (`self.PointLight`) false false)
      (set `self.activated` false))))

(fn `UserConstructionScript`
  (`parent.UserConstructionScript`))