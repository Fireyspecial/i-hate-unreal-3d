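; BP_Robber is the player character for a stealth game, with crouch, roll, mantle, guard takedowns, interaction, pause menu and ragdoll.
; Crouch timelines blend capsule, mesh and camera arm, and a sphere trace blocks standing under obstacles.
; Mantle scans upward then down for a ledge, picking a one- or two-meter montage by distance.
; Motion warping aligns mantles and takedowns, with interface calls on overlapping actors driving interactions and takedowns.
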(event `self.ReceiveBeginPlay`
  ;[1 1 1] Input and Movement
  (`EnhancedInputSubsystemInterface.AddMappingContext` (pcsubsystem `EnhancedInputLocalPlayerSubsystem` (`GameplayStatics.GetPlayerController` 0)) "/Game/Input/IMC_MappingContext.IMC_MappingContext" 0 (struct))
  (bind _returnvalue (`|CreateWidget` "/Game/UI/WB_DetectionMeter.WB_DetectionMeter_C"))
  (bind _output_get (set `self.Detected Meter Widget` _returnvalue))
  (`UserWidget.AddToViewport` _output_get 0))

(event `EnhancedInput|/Game/Input/IA_Move`
  (params (ActionValue :type "Vector2D Structure") (ElapsedSeconds :type "Float (double-precision)") (TriggeredSeconds :type "Float (double-precision)") (InputAction :type "InputAction Object Reference" :default "/Game/Input/IA_Move.IA_Move"))
  ;[1 1 1] Input and Movement
  (:`Triggered`
    (`self.AddMovementInput` (`KismetMathLibrary.GetRightVector` (`self.GetControlRotation`)) ActionValue_X)
    (`self.AddMovementInput` (`KismetMathLibrary.GetForwardVector` (`self.GetControlRotation`)) ActionValue_Y)))

(event `EnhancedInput|/Game/Input/IA_Look`
  (params (ActionValue :type "Vector2D Structure") (ElapsedSeconds :type "Float (double-precision)") (TriggeredSeconds :type "Float (double-precision)") (InputAction :type "InputAction Object Reference" :default "/Game/Input/IA_Look.IA_Look"))
  ;[1 1 1] Input and Movement
  (:`Triggered`
    (`self.AddControllerYawInput` ActionValue_X)
    (`self.AddControllerPitchInput` (* ActionValue_Y -1.0))))

(event `EnhancedInput|/Game/Input/IA_Crouch`
  (params (ActionValue :type Boolean) (ElapsedSeconds :type "Float (double-precision)") (TriggeredSeconds :type "Float (double-precision)") (InputAction :type "InputAction Object Reference" :default "/Game/Input/IA_Crouch.IA_Crouch"))
  (bind _charactermovement (`self.CharacterMovement`))
  ;[1 1 1] Crouch
  (:`Started`
    (if (not (`self.crouched`))
      (set `self.crouched` true)
      (set `CharacterMovementComponent.MaxWalkSpeed` 350.0 _charactermovement)
      (`|ExecutionSequence`
        (:`then_0`
          (bind (_direction _arm_length) (`Timeline|Crouch Zoom Out` :!label _label)
            (:`Update`
              (set `SpringArmComponent.TargetArmLength` (`KismetMathLibrary.Lerp` 600.0 750.0 _arm_length) (`self.SpringArm`)))))
        (:`then_1`
          (bind (_direction_2 _capsule_height) (`Timeline|Capsule Height` :!label _label_2)
            (:`Update`
              (`CapsuleComponent.SetCapsuleHalfHeight` (`self.CapsuleComponent`) (`KismetMathLibrary.Lerp` 88.0 50.0 _capsule_height) true)
              (`SceneComponent.K2_SetRelativeLocation` (`self.Mesh`) (`KismetMathLibrary.MakeVector` 0.0 0.0 (`KismetMathLibrary.Lerp` -89.0 -59.0 _capsule_height)) false false)))))
      (else
        (bind _hit_ (`self.Uncrouch Obstacle Detection`))
        (if (not _hit_)
          (set `self.crouched` false)
          (set `CharacterMovementComponent.MaxWalkSpeed` 600.0 _charactermovement)
          (`|ExecutionSequence`
            (:`then_0`
              (goto _label :!via `Reverse`))
            (:`then_1`
              (goto _label_2 :!via `Reverse`))))))))

(event `EnhancedInput|/Game/Input/IA_Interact`
  (params (ActionValue :type Boolean) (ElapsedSeconds :type "Float (double-precision)") (TriggeredSeconds :type "Float (double-precision)") (InputAction :type "InputAction Object Reference" :default "/Game/Input/IA_Interact.IA_Interact"))
  ;[1 1 1] Interactions and Stealth Takedown
  (:`Started`
    (`|ExecutionSequence`
      (:`then_0`
        (for _array_element (`self.GetOverlappingActors` null)
          (if (`KismetSystemLibrary.DoesImplementInterface` _array_element "/Game/Blueprints/BPI_Interact.BPI_Interact_C")
            (message `/Game/Blueprints/BPI_Interact.Interact` _array_element))))
      (:`then_1`
        (for _array_element_2 (`self.GetOverlappingActors` null)
          (if (`KismetSystemLibrary.DoesImplementInterface` _array_element_2 "/Game/Blueprints/BPI_Guard.BPI_Guard_C")
            (bind (_ref_pose _rotation _can_takedown _actor) (message `/Game/Blueprints/BPI_Guard.Takedown` _array_element_2))
            (if _can_takedown
              (`|PlayMontage` (`self.Mesh`) "/Game/Characters/Robber/Takedowns/Takedown_Attacker_Montage.Takedown_Attacker_Montage"
                (:`then`
                  (`MotionWarpingComponent.AddOrUpdateWarpTarget` (`self.MotionWarping`) (make `MotionWarpingTarget` "Takedown" _ref_pose _rotation))
                  (`PrimitiveComponent.IgnoreActorWhenMoving` (`self.Mesh`) _actor true)
                  (`PrimitiveComponent.IgnoreActorWhenMoving` (`self.CapsuleComponent`) _actor true))))))))))

(event `EnhancedInput|/Game/Input/IA_Roll`
  (params (ActionValue :type Boolean) (ElapsedSeconds :type "Float (double-precision)") (TriggeredSeconds :type "Float (double-precision)") (InputAction :type "InputAction Object Reference" :default "/Game/Input/IA_Roll.IA_Roll"))
  ;[1 1 1] Dodge Roll
  (:`Started`
    (if (not (`self.is dodging?`))
      (`|PlayMontage` (`self.Mesh`) "/Game/Characters/Robber/Roll/Roll_Montage.Roll_Montage"
        (:`then`
          (set `self.is dodging?` true))
        (:`OnCompleted`
          (set `self.is dodging?` false))))))

(event `EnhancedInput|/Game/Input/IA_Mantle`
  (params (ActionValue :type Boolean) (ElapsedSeconds :type "Float (double-precision)") (TriggeredSeconds :type "Float (double-precision)") (InputAction :type "InputAction Object Reference" :default "/Game/Input/IA_Mantle.IA_Mantle"))
  (bind (_returnvalue_x _returnvalue_y) (`KismetMathLibrary.BreakVector` (`self.GetActorForwardVector`)))
  (:`Started`
    (if (and (not (`self.mantling`)) (not (`NavMovementComponent.IsFalling` (`self.CharacterMovement`))))
      (for _index (range (+ (`KismetMathLibrary.SelectInt` 7 4 (`self.crouched`)) 1))
        (bind _returnvalue (+ (`self.K2_GetActorLocation`) (`KismetMathLibrary.MakeVector` 0.0 0.0 (* _index 30))))
        (bind (_outhit _returnvalue_2) (`KismetSystemLibrary.SphereTraceSingle` :`Start` _returnvalue :`End` (+ _returnvalue (* (`KismetMathLibrary.GetForwardVector` (`self.K2_GetActorRotation`)) 120.0)) :`Radius` 7.0 :`TraceChannel` "TraceTypeQuery1" :`DrawDebugType` "ForDuration"))
        (if (not _returnvalue_2)
          (`|ExecutionSequence`
            (:`then_0`
              (if (!= _index 0)
                (for _index_2 (range 5)
                  (bind _returnvalue_3 (+ (`self.K2_GetActorLocation`) (`KismetMathLibrary.MakeVector` (* (* _index_2 20) _returnvalue_x) (* _returnvalue_y (* _index_2 20)) 200.0)))
                  (bind (_outhit_2 _returnvalue_4) (`KismetSystemLibrary.SphereTraceSingle` :`Start` _returnvalue_3 :`End` (+ _returnvalue_3 (* (`self.GetActorUpVector`) -200.0)) :`Radius` 7.0 :`TraceChannel` "TraceTypeQuery1" :`DrawDebugType` "ForDuration"))
                  (if _returnvalue_4
                    (`|ExecutionSequence`
                      (:`then_0`
                        (bind (_bblockinghit _binitialoverlap _time _distance _location) (`GameplayStatics.BreakHitResult` _outhit_2))
                        (`KismetSystemLibrary.DrawDebugSphere` _location 10.0 12 (struct :`R` 0.187984 :`G` 1.0 :`A` 1.0) 100000.0 2.0)
                        (`MotionWarpingComponent.AddOrUpdateWarpTarget` (`self.MotionWarping`) (make `MotionWarpingTarget` "Mantle" (+ _location (0.0 0.0 -3.0)) (`self.K2_GetActorRotation`)))
                        (if (> (`KismetMathLibrary.Vector_Distance` _location (`SceneComponent.K2_GetComponentLocation` (`self.Mesh`))) 200.0)
                          (`KismetSystemLibrary.PrintString` "2 Meter")
                          (`|PlayMontage` (`self.Mesh`) "/Game/Characters/Robber/Mantling/Mantling_2M_Montage.Mantling_2M_Montage"
                            (:`then`
                              (`CharacterMovementComponent.SetMovementMode` (`self.CharacterMovement`) "MOVE_Flying" 0 :!label _label_3)
                              (set `self.mantling` true)
                              (if (`self.crouched`)
                                (`CapsuleComponent.SetCapsuleHalfHeight` (`self.CapsuleComponent`) 88.0 true)
                                (`SceneComponent.K2_SetRelativeLocation` (`self.Mesh`) (0.0 0.0 -89.0) false false)))
                            (:`OnCompleted`
                              (set `self.mantling` false :!label _label_4)
                              (`CharacterMovementComponent.SetMovementMode` (`self.CharacterMovement`) "MOVE_Walking" 0)
                              (if (`self.crouched`)
                                (bind (_direction _capsule_height) (`Timeline|Timeline`)
                                  (:`Update`
                                    (`CapsuleComponent.SetCapsuleHalfHeight` (`self.CapsuleComponent`) (`KismetMathLibrary.Lerp` 88.0 50.0 _capsule_height) true)
                                    (`SceneComponent.K2_SetRelativeLocation` (`self.Mesh`) (`KismetMathLibrary.MakeVector` 0.0 0.0 (`KismetMathLibrary.Lerp` -89.0 -59.0 _capsule_height)) false false))))))
                          (else
                            (`KismetSystemLibrary.PrintString` "1 Meter")
                            (`|PlayMontage` (`self.Mesh`) "/Game/Characters/Robber/Mantling/Mantling_1M_Montage.Mantling_1M_Montage"
                              (:`then`
                                (goto _label_3))
                              (:`OnCompleted`
                                (goto _label_4))))))
                      (:`then_1`
                        (break)))))))
            (:`then_1`
              (break))))))))

(event `Ragdoll`
  (`PrimitiveComponent.SetSimulatePhysics` (`self.Mesh`) true)
  (`self.DisableInput` null))

(event `EnhancedInput|/Game/Input/IA_Pause`
  (params (ActionValue :type Boolean) (ElapsedSeconds :type "Float (double-precision)") (TriggeredSeconds :type "Float (double-precision)") (InputAction :type "InputAction Object Reference" :default "/Game/Input/IA_Pause.IA_Pause"))
  (bind _returnvalue (`GameplayStatics.GetPlayerController` 0))
  (bind _returnvalue_2 (`GameplayStatics.GetPlayerController` 0))
  (:`Triggered`
    (if (not (`self.paused?`))
      (set `self.paused?` true)
      (bind _returnvalue_3 (`|CreateWidget` "/Game/UI/WB_PauseMenu.WB_PauseMenu_C"))
      (bind _output_get (set `self.PauseMenuWB` _returnvalue_3))
      (`UserWidget.AddToViewport` _output_get 0)
      (set `PlayerController.bShowMouseCursor` true _returnvalue_2)
      (`WidgetBlueprintLibrary.SetInputMode_GameAndUIEx` _returnvalue_2 (`self.PauseMenuWB`))
      (`GameplayStatics.SetGamePaused` true)
      (else
        (bind _pausemenuwb (`self.PauseMenuWB` :!label _label_5)
          (:`then`
            (`Widget.RemoveFromParent` _pausemenuwb)
            (set `self.PauseMenuWB` null)
            (set `self.paused?` false)
            (set `PlayerController.bShowMouseCursor` false _returnvalue)
            (`WidgetBlueprintLibrary.SetInputMode_GameOnly` _returnvalue)
            (`GameplayStatics.SetGamePaused` false))
          (:`else`))))))

(event `Resume`
  (goto _label_5))

(fn `Uncrouch Obstacle Detection`
  (returns (`Hit?` :type Boolean))
  (bind _returnvalue (`self.K2_GetActorLocation`))
  (bind (_outhit _returnvalue_2) (`KismetSystemLibrary.SphereTraceSingle` :`Start` _returnvalue :`End` (+ _returnvalue (* (`KismetMathLibrary.GetUpVector` (`self.K2_GetActorRotation`)) 115.0)) :`Radius` 15.0 :`TraceChannel` "TraceTypeQuery1" :`DrawDebugType` "ForDuration"))
  (return _returnvalue_2))

(fn `UserConstructionScript`)